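; BP_OcTreePoint is an actor that visualizes a single octree point as a sphere with an ID label.
; On BeginPlay it scales the sphere from its Range and passes its Id to the UMG_NodeId widget.
; Activate and Deactivate events toggle a highlight by setting the sphere material's Color parameter to amber or white.
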(event `self.ReceiveBeginPlay`
  (`SceneComponent.SetWorldScale3D` (`self.Sphere`) (`KismetMathLibrary.Conv_DoubleToVector` (/ (`self.Range`) 100.0)))
  (`/Game/QuadTree/UMG_NodeId.SetID` (cast `/Game/QuadTree/UMG_NodeId` (`WidgetComponent.GetWidget` (`self.Widget`)) :!pure true) (`self.id`)))

(event `self.Activate`
  (`MeshComponent.SetVectorParameterValueOnMaterials` (`self.Sphere`) "Color" (1.0 0.73 0.0)))

(event `self.Deactivate`
  (`MeshComponent.SetVectorParameterValueOnMaterials` (`self.Sphere`) "Color" (1.0 1.0 1.0)))

(fn `UserConstructionScript`)